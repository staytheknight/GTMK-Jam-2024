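; BP_Leaf is an obstacle that becomes destroyable when a large enough BP_Swarm overlaps it.
; LeafCollision overlap events maintain a list of swarms, filtered to static mesh components.
; Each tick sets CanBeDestroyed if any single swarm meets SwarmSizeNeeded, while a widget shows the shortfall against the combined size of all overlapping swarms.
; The destruction itself happens outside these graphs.
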(event OnComponentBeginOverlap(LeafCollision)
  (params (OverlappedComponent :type Primitive%20Component%20Object%20Reference) (OtherActor :type Actor%20Object%20Reference) (OtherComp :type Primitive%20Component%20Object%20Reference) (OtherBodyIndex :type Integer) (bFromSweep :type Boolean) (SweepResult :type Hit%20Result%20Structure%20%28by%20ref%29))
  (if (== (Utilities|GetClass OtherComp) "/Script/Engine.StaticMeshComponent")
    (bind _asbp_swarm (Utilities|Casting|CastToBP_Swarm OtherActor))
    (Utilities|Array|AddUnique (Variables|Default|GetOverlaped%20Swarms) _asbp_swarm)))

(event OnComponentEndOverlap(LeafCollision)
  (params (OverlappedComponent :type Primitive%20Component%20Object%20Reference) (OtherActor :type Actor%20Object%20Reference) (OtherComp :type Primitive%20Component%20Object%20Reference) (OtherBodyIndex :type Integer))
  (if (== (Utilities|GetClass OtherComp) "/Script/Engine.StaticMeshComponent")
    (bind _asbp_swarm (Utilities|Casting|CastToBP_Swarm OtherActor))
    (Utilities|Array|RemoveItem (Variables|Default|GetOverlaped%20Swarms) _asbp_swarm)))

(event EventTick
  (params (DeltaSeconds :type Float%20%28single-precision%29))
  (CallFunction|UpdateWidget)
  (CallFunction|CheckOverlapListforProperSizedSwarm))

(fn ConstructionScript
  (|CallParentFunction))

(fn CheckOverlapListforProperSizedSwarm
  (Utilities|Array|Clear (LocalVariables|GetLargeEnoughSwarmExists))
  (for _array_element (Variables|Default|GetOverlaped%20Swarms)
    (Utilities|IsValid _array_element
      (:Is%20Valid
        (Utilities|Array|Add (LocalVariables|GetLargeEnoughSwarmExists) (>= (Variables|/Game/Blueprints/Core/Swarm/BP_Swarm.BP_Swarm_C|GetSwarmSize _array_element) (Variables|Default|GetSwarm%20Size%20Needed))))))
  (Variables|Default|SetcanBeDestroyed (Utilities|Array|ContainsItem (LocalVariables|GetLargeEnoughSwarmExists) true)))

(fn UpdateWidget
  (bind _asw_swarm_size_needed (Utilities|Casting|CastToW_SwarmSizeNeededToOpen (UserInterface|GetWidget (Variables|Default|GetSwarm%20Size%20Needed%20Widget))))
  (for _array_element (Variables|Default|GetOverlaped%20Swarms)
    (Utilities|IsValid _array_element
      (:Is%20Valid
        (LocalVariables|SetSwarmSizeOverlapped (+ (LocalVariables|GetSwarmSizeOverlapped) (Variables|/Game/Blueprints/Core/Swarm/BP_Swarm.BP_Swarm_C|GetSwarmSize _array_element))))))
  (Variables|/Game/Blueprints/Core/UI/W_SwarmSizeNeededToOpen.W_SwarmSizeNeededToOpen_C|SetSwarmSize _asw_swarm_size_needed (Math|Integer|Clamp(Integer) (- (Variables|Default|GetSwarm%20Size%20Needed) (LocalVariables|GetSwarmSizeOverlapped)) 0 (- (Variables|Default|GetSwarm%20Size%20Needed) (LocalVariables|GetSwarmSizeOverlapped)))))