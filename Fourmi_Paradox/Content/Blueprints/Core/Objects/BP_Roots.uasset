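; BP_Roots is a roots object that breaks into a BP_Swarm once all its attached leaves can be destroyed.
; The construction script gathers child actor components, turns the configured number into BP_Leaf actors and gives each its required swarm size.
; Tick polls every leaf's CanBeDestroyed flag.
; When none is false, it spawns an enlarged swarm of configured size at the roots' location and destroys itself.
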(event EventTick
  (params (DeltaSeconds :type Float%20%28single-precision%29))
  (Utilities|Array|Clear (Variables|Default|GetcanLeavesBeDestroyed))
  ;[1 1 1] Every tick go through all the leaves connected to the roots, and check their 'can be destroyed flag', add it to a boolean array
  (bind _array_element (Utilities|Array|ForEachLoopwithBreak (Variables|Default|GetLeafs))
    (:LoopBody
      (bind _asbp_leaf (Utilities|Casting|CastToBP_Leaf (Variables|/Script/Engine.ChildActorComponent|GetChildActor _array_element)))
      (Utilities|Array|Add (Variables|Default|GetcanLeavesBeDestroyed) (Variables|/Game/Blueprints/Core/Objects/BP_Leaf.BP_Leaf_C|GetcanBeDestroyed _asbp_leaf)))
    (:Completed
      ;[1 1 1] If it does not contain any 'false' 'can be destroyed' flags - destroy the roots
      (if (not (Utilities|Array|ContainsItem (Variables|Default|GetcanLeavesBeDestroyed) false))
        (Game|SpawnActorfromClass "/Game/Blueprints/Core/Swarm/BP_Swarm.BP_Swarm_C" (Math|Transform|MakeTransform (Transformation|GetWorldLocation (Variables|Default|GetDefaultSceneRoot self)) "0, 0, 0" "2.000000,2.000000,2.000000") "AdjustIfPossibleButAlwaysSpawn" "MultiplyWithRoot" 0 (Variables|Default|GetswarmSizeToSpawn) 0)
        (Actor|DestroyActor)))))

(fn ConstructionScript
  (for _array_element (Actor|GetComponentsByClass "/Script/Engine.ChildActorComponent")
    (Utilities|Array|Add (Variables|Default|GetLeafs) _array_element)
    (CallFunction|SpawnLeaves (Variables|Default|GetNumberOfLeavesToSpawn))))

(fn SpawnLeaves
  (params (NumberOfLeaves :type Integer))
  (for _index (range 0 (- NumberOfLeaves 1))
    (ChildActorComponent|SetChildActorClass (Utilities|Array|Get(acopy) (Variables|Default|GetLeafs) _index) "/Game/Blueprints/Core/Objects/BP_Leaf.BP_Leaf_C")
    (bind _asbp_leaf (Utilities|Casting|CastToBP_Leaf (Variables|/Script/Engine.ChildActorComponent|GetChildActor (Utilities|Array|Get(acopy) (Variables|Default|GetLeafs) _index))))
    (Variables|/Game/Blueprints/Core/Objects/BP_Leaf.BP_Leaf_C|SetSwarm%20Size%20Needed _asbp_leaf (Utilities|Array|Get(acopy) (Variables|Default|GetswarmSizeNeededForLeaves) _index))))