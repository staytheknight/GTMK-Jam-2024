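; BP_Food is a food object that delivers itself to the hive once flagged ReadyForHive, deferring to its parent class's Tick until then.
; After a short BeginPlay delay it caches the first BP_Hive in the level.
; When ready, Tick hides the pickup, drop and swarm-size prompts and interpolates the food toward the hive mouth.
; Within a distance tolerance of the mouth, it increments the hive's FoodDelivered count and destroys itself.
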(event EventBeginPlay
  (|CallParentFunction)
  (Utilities|FlowControl|Delay 0.2)
  (bind _outactors (Actor|GetAllActorsOfClass "/Game/Blueprints/Core/Objects/BP_Hive.BP_Hive_C"))
  (Variables|Default|SetBP_Hive (Utilities|Array|Get(acopy) _outactors)))

(event Collision|EventActorBeginOverlap
  (params (OtherActor :type Actor%20Object%20Reference))
  (|CallParentFunction OtherActor) ; This node is disabled and will not be called.\nDrag off pins to build functionality.
)

(event EventTick
  (params (DeltaSeconds :type Float%20%28single-precision%29))
  (if (Variables|Default|GetreadyForHive)
    (Development|SetHiddeninGame (Variables|Default|GetPickUpPrompt) true false)
    (CallFunction|MoveFoodtoHiveMouth)
    (CallFunction|DestroyFood 1e+02)
    (else
      (|CallParentFunction DeltaSeconds))))

(fn ConstructionScript
  (|CallParentFunction))

(fn MoveFoodtoHiveMouth
  (bind _defaultsceneroot (Variables|Default|GetDefaultSceneRoot))
  (bind _bp_hive (Variables|Default|GetBP_Hive))
  (bind _defaultsceneroot_2 (Variables|/Game/Blueprints/Core/Objects/BP_Hive.BP_Hive_C|GetDefaultSceneRoot _bp_hive))
  (bind _returnvalue (Transformation|GetWorldLocation _defaultsceneroot_2))
  (Transformation|SetWorldLocation _defaultsceneroot (Math|Interpolation|VInterpTo (Transformation|GetWorldLocation _defaultsceneroot) (Math|Vector|MakeVector (.x _returnvalue) (.y _returnvalue) (+ (.z _returnvalue) (Variables|Default|GetHiveMouthZLoc))) (Utilities|Time|GetWorldDeltaSeconds) (Variables|Default|GetDeliverToHiveInterpSpeed)) false false))

(fn DestroyFood
  (params (DistanceTolerance :type Float%20%28double-precision%29))
  (bind _bp_hive (Variables|Default|GetBP_Hive))
  (bind _rootcomponent (Variables|/Script/Engine.Actor|GetRootComponent _bp_hive))
  (bind _returnvalue (Transformation|GetWorldLocation _rootcomponent))
  (if (< (Math|Vector|Distance(Vector) (Transformation|GetWorldLocation (Variables|Default|GetDefaultSceneRoot)) (Math|Vector|MakeVector (.x _returnvalue) (.y _returnvalue) (+ (.z _returnvalue) (Variables|Default|GetHiveMouthZLoc)))) DistanceTolerance)
    (Math|Integer|IncrementInt (Variables|/Game/Blueprints/Core/Objects/BP_Hive.BP_Hive_C|GetFoodDelivered (Variables|Default|GetBP_Hive))
      (:%20%20
        (Actor|DestroyActor)))))