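; BP_Hive is the hive actor that marks dropped-off BP_Food as ready for the hive.
; Shortly after BeginPlay it stores the count of all BP_Food actors in the level as FoodNeeded, which this file does not otherwise use.
; Its SphereCollider overlap events maintain a list of food inside the sphere.
; Every Tick, SetReadyFood sets ReadyForHive on each valid listed food that is not being carried.
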(event OnComponentBeginOverlap(SphereCollider)
  (params (OverlappedComponent :type Primitive%20Component%20Object%20Reference) (OtherActor :type Actor%20Object%20Reference) (OtherComp :type Primitive%20Component%20Object%20Reference) (OtherBodyIndex :type Integer) (bFromSweep :type Boolean) (SweepResult :type Hit%20Result%20Structure%20%28by%20ref%29))
  (bind _asbp_food (Utilities|Casting|CastToBP_Food OtherActor))
  (Utilities|Array|AddUnique (Variables|Default|GetFoodOverlaping) _asbp_food))

(event OnComponentEndOverlap(SphereCollider)
  (params (OverlappedComponent :type Primitive%20Component%20Object%20Reference) (OtherActor :type Actor%20Object%20Reference) (OtherComp :type Primitive%20Component%20Object%20Reference) (OtherBodyIndex :type Integer))
  (bind _asbp_food (Utilities|Casting|CastToBP_Food OtherActor))
  (Utilities|Array|RemoveItem (Variables|Default|GetFoodOverlaping) _asbp_food))

(event EventBeginPlay
  (Utilities|FlowControl|Delay 0.2)
  (bind _outactors (Actor|GetAllActorsOfClass "/Game/Blueprints/Core/Objects/BP_Food.BP_Food_C"))
  (Variables|Default|SetFoodNeeded (Utilities|Array|Length _outactors)))

(event Collision|EventActorBeginOverlap
  (params (OtherActor :type Actor%20Object%20Reference)))

(event EventTick
  (params (DeltaSeconds :type Float%20%28single-precision%29))
  (CallFunction|SetReadyFood))

(fn ConstructionScript)

(fn SetReadyFood
  (for _array_element (Variables|Default|GetFoodOverlaping)
    (bind _output_get (LocalVariables|SetArrayElement _array_element))
    (Utilities|IsValid _output_get
      (:Is%20Valid
        (if (not (Variables|/Game/Blueprints/Core/Objects/BP_MoveableObject.BP_MoveableObject_C|GetisBeingCarried _output_get))
          (Variables|/Game/Blueprints/Core/Objects/BP_Food.BP_Food_C|SetreadyForHive (LocalVariables|GetArrayElement) true))))))