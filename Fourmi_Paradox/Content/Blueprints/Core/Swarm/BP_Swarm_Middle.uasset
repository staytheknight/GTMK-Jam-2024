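; BP_Swarm_Middle is the connecting body of a swarm, a mesh that spans the gap between a Head and a Tail.
; Every tick, Stretch checks both references, scales the mesh's X to their distance, matches Y to the head's mesh and keeps Z thin.
; It then moves its root to the midpoint between the two.
; Rotation is not set in this Blueprint.
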(event EventTick
  (params (DeltaSeconds :type Float%20%28single-precision%29))
  (CallFunction|Stretch))

(fn ConstructionScript)

(fn Stretch
  (bind _head (Variables|Default|GetHead))
  (bind _tail (Variables|Default|GetTail))
  (bind _defaultsceneroot (Variables|/Game/Blueprints/Core/Swarm/BP_Swarm.BP_Swarm_C|GetDefaultSceneRoot _head))
  (bind _defaultsceneroot_2 (Variables|/Game/Blueprints/Core/Swarm/BP_Swarm_Tail.BP_Swarm_Tail_C|GetDefaultSceneRoot _tail))
  (bind _returnvalue (Transformation|GetWorldLocation _defaultsceneroot))
  (bind _returnvalue_2 (Transformation|GetWorldLocation _defaultsceneroot_2))
  (Utilities|IsValid _head
    (:Is%20Valid
      (Utilities|IsValid _tail
        (:Is%20Valid
          (Transformation|SetWorldScale3D (Variables|Default|GetSM_Swarm_Middle) (Math|Vector|MakeVector (/ (Math|Vector|Distance(Vector) _returnvalue _returnvalue_2) 1e+02) (.y (Transformation|GetWorldScale (Variables|/Game/Blueprints/Core/Swarm/BP_Swarm.BP_Swarm_C|GetSM_Swarm _head))) 0.025))
          (Transformation|SetWorldLocation (Variables|Default|GetDefaultSceneRoot) (/ (+ _returnvalue _returnvalue_2) 2) false false))))))