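; Swarm ant actor that walks toward a Target point and wanders intermittently once within TargetDistance.
; Each unfrozen tick blends target direction with random sideways wiggle, yawing by capped steps using dot product for angle and cross product for sign.
; A downward trace ahead permits forward movement only over ground.
; Near the target, random rolls start and stop wandering; TeleportToTarget snaps the ant to Target.
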(event EventTick
  (params (DeltaSeconds :type Float%20%28single-precision%29))
  (bind _returnvalue (Transformation|GetActorLocation))
  (bind _returnvalue_2 (Transformation|GetActorLocation))
  (bind _returnvalue_3 (Transformation|GetActorRotation))
  (bind _returnvalue_4 (Transformation|GetActorLocation))
  (bind _returnvalue_5 (Transformation|GetActorRotation))
  (bind _target (Variables|Default|GetTarget))
  (bind _targetdistance (Variables|Default|GetTargetDistance))
  (bind _wiggleamount (Variables|Default|GetWiggleAmount))
  (bind _target_2 (Variables|Default|GetTarget))
  (bind _returnvalue_6 (Math|Vector|Distance(Vector) _target _returnvalue))
  (bind _returnvalue_7 (Math|Vector|GetForwardVector _returnvalue_5))
  (bind _returnvalue_8 (Math|Vector|GetRightVector _returnvalue_3))
  (bind _returnvalue_9 (Math|Vector|GetForwardVector _returnvalue_3))
  (bind _returnvalue_10 (* _wiggleamount -1.0))
  (bind _returnvalue_11 (- _target_2 _returnvalue_4))
  (bind _returnvalue_12 (Math|Vector2D|MakeVector2D (.x _returnvalue_9) (.y _returnvalue_9)))
  (bind _returnvalue_13 (Math|Random|RandomFloatinRange _wiggleamount _returnvalue_10))
  (bind _returnvalue_14 (> _returnvalue_6 _targetdistance))
  (bind _returnvalue_15 (* _returnvalue_7 1e+02))
  (bind _returnvalue_16 (Math|Vector2D|Normalize2D _returnvalue_12))
  (bind _returnvalue_17 (Math|Conversions|ToFloat(Boolean) _returnvalue_14))
  (bind _returnvalue_18 (+ _returnvalue_2 _returnvalue_15))
  (bind _returnvalue_19 (* _returnvalue_8 _returnvalue_13))
  (bind _returnvalue_20 (* _returnvalue_11 _returnvalue_17))
  (bind _returnvalue_21 (+ _returnvalue_19 _returnvalue_20))
  (bind _returnvalue_22 (Math|Conversions|ToVector2D(Vector) _returnvalue_21))
  (bind _returnvalue_23 (Math|Vector2D|Normalize2D _returnvalue_22))
  (bind _returnvalue_24 (Math|Vector2D|DotProduct(2D) _returnvalue_16 _returnvalue_23))
  (bind _returnvalue_25 (Class|KismetMathLibrary|DegAcos _returnvalue_24))
  ;[1 1 1] Test if a spot ahead of the ant is on ground
  (bind _returnvalue_26 (Collision|LineTraceForObjects _returnvalue_18 (- _returnvalue_18 "0.000000,0.000000,500.000000") (Utilities|Array|MakeArray "ObjectTypeQuery1") false 0 "None"))
  (Variables|Default|SetGroundAhead _returnvalue_26)
  (if (not (Variables|Default|GetFrozen))
    (Variables|Default|SetWanderTime (+ (* DeltaSeconds (Math|Conversions|ToFloat(Boolean) (not _returnvalue_14))) (Variables|Default|GetWanderTime)))
    (if (not (and (not _returnvalue_14) false))
      (if (or _returnvalue_14 (Variables|Default|GetWalking))
        ;[1 1 1] Calculate how the actor has to rotate to align with calculated direction vector
        (if (> _returnvalue_25 1e+01)
          (Transformation|AddActorLocalRotation (Math|Rotator|MakeRotator 0.0 0.0 (* (Math|Float|Min(Float) (Variables|Default|GetTurnSpeed) _returnvalue_25) (Math|Float|Sign(Float) (Class|KismetMathLibrary|CrossProduct2D _returnvalue_16 _returnvalue_23)))) false false))
        (if (or false (Variables|Default|GetGroundAhead))
          (Transformation|SetActorLocation (+ (* (Math|Vector|GetForwardVector (Transformation|GetActorRotation)) (Variables|Default|GetWalkSpeed)) (Transformation|GetActorLocation)) false false)
          (if (and (< (Math|Random|RandomFloat) 0.05) (> (Variables|Default|GetWanderTime) 2.0))
            (Variables|Default|SetWalking false)
            (Variables|Default|SetWanderTime 0.0)))
        (else
          ;[1 1 1] Decide if the ant wants to wander
          (Variables|Default|SetWalking (<= (Math|Random|RandomFloat) (Variables|Default|GetWanderChance))))))))

(fn ConstructionScript)

(fn TeleporttoTarget
  (Transformation|SetActorLocation (Variables|Default|GetTarget) false false))