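; Swarm manager that spawns BP_Ant actors, shares the list and a target with them, and destroys them with itself.
; MakeBridge spaces slots evenly between two points, which UpdateBridge recomputes.
; While bridging, Tick freezes ants within range of the manager's Target and manually steps them into slots.
; RemoveBridge teleports stragglers to the end position, while Tick walks bridged ants there before unfreezing them.
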(event EventDestroyed
  (for _array_element (Variables|Default|GetAnts)
    (Actor|DestroyActor _array_element)))

(event EventTick
  (params (DeltaSeconds :type Float%20%28single-precision%29))
  (bind _bridgeend (Variables|Default|GetBridgeEnd))
  (if (Variables|Default|GetBridging)
    ;[1 1 1] Check if ants are in a position where they can start bridging (don't want them too spread out or the bridge might not construct)
    (bind (_arrayindex _arrayelement) (Utilities|Array|ReverseforEachLoop (Variables|Default|GetAntsNotAtBridge))
      (:LoopBody
        (if (<= (Math|Vector|Distance2D(Vector) (Math|Conversions|ToVector2D(Vector) (Transformation|GetActorLocation _arrayelement)) (Math|Conversions|ToVector2D(Vector) (Variables|Default|GetTarget))) 1.5e+02)
          (Utilities|Array|Add (Variables|Default|GetAntsBridging) _arrayelement)
          (Variables|/Game/Blueprints/Core/Swarm/BP_Ant.BP_Ant_C|SetFrozen _arrayelement true)
          (Utilities|Array|RemoveIndex (Variables|Default|GetAntsNotAtBridge) _arrayindex)))
      (:Completed
        ;[1 1 1] Manually move ants to their target positions
        (for (_array_element _array_index) (Variables|Default|GetAntsBridging)
          (Transformation|AddActorWorldOffset _array_element (* (Math|Vector|Normalize (- (Utilities|Array|Get(acopy) (Variables|Default|GetBridgePositions) _array_index) (Transformation|GetActorLocation _array_element))) (Math|Float|Min(Float) 5e+01 (Math|Vector|Distance(Vector) (Utilities|Array|Get(acopy) (Variables|Default|GetBridgePositions) _array_index) (Transformation|GetActorLocation _array_element))))))))
    (else
      ;[1 1 1] Check if ants are in a position where they are off the bridge and can be removed from manual control
      (bind (_arrayindex_2 _arrayelement_2) (Utilities|Array|ReverseforEachLoop (Variables|Default|GetAntsBridging))
        (:LoopBody
          (if (<= (Math|Vector|Distance2D(Vector) (Math|Conversions|ToVector2D(Vector) (Transformation|GetActorLocation _arrayelement_2)) (Math|Conversions|ToVector2D(Vector) (Variables|Default|GetBridgeEnd))) 5e+01)
            (Variables|/Game/Blueprints/Core/Swarm/BP_Ant.BP_Ant_C|SetFrozen _arrayelement_2 false)
            (Utilities|Array|RemoveIndex (Variables|Default|GetAntsBridging) _arrayindex_2)))
        (:Completed
          ;[1 1 1] Manually move ants to their target positions
          (for _array_element_2 (Variables|Default|GetAntsBridging)
            (Transformation|AddActorWorldOffset _array_element_2 (* (Math|Vector|Normalize (- _bridgeend (Transformation|GetActorLocation _array_element_2))) (Math|Float|Min(Float) 5e+01 (Math|Vector|Distance(Vector) _bridgeend (Transformation|GetActorLocation _array_element_2))))))
          ;[1 1 1] If we aren't bridging just make sure all ants know the target location
          (for _array_element_3 (Variables|Default|GetAnts)
            (Variables|/Game/Blueprints/Core/Swarm/BP_Ant.BP_Ant_C|SetTarget _array_element_3 (Variables|Default|GetTarget))))))))

(fn ConstructionScript)

(fn SpawnAnts
  (params (Amount :type Integer))
  (for _index (range 1 Amount)
    (bind _returnvalue (Game|SpawnActorfromClass "/Game/Blueprints/Core/Swarm/BP_Ant.BP_Ant_C" (Transformation|GetActorTransform) "Undefined" "MultiplyWithRoot" 0 0))
    (Utilities|Array|Add (Variables|Default|GetAnts) _returnvalue))
  (for _array_element (Variables|Default|GetAnts)
    (Variables|/Game/Blueprints/Core/Swarm/BP_Ant.BP_Ant_C|SetAnts _array_element (Variables|Default|GetAnts))))

(fn MakeBridge
  (params (Start :type Vector) (End :type Vector))
  (bind _ants (Variables|Default|GetAnts))
  (bind _returnvalue (Utilities|Array|Length _ants))
  (bind _returnvalue_2 (- _returnvalue 1))
  (Variables|Default|SetBridgeStart Start)
  (Variables|Default|SetBridgeEnd End)
  (Variables|Default|SetBridging true)
  ;[1 1 1] Calculate the ant positions along the bridge
  (for _index (range 0 _returnvalue_2)
    (Utilities|Array|Add (Variables|Default|GetBridgePositions) (Math|Vector|Lerp(Vector) (Variables|Default|GetBridgeStart) (Variables|Default|GetBridgeEnd) (/ _index _returnvalue_2))))
  ;[1 1 1] Add all ants to the 'not at bridge' array
  (Utilities|Array|Clear (Variables|Default|GetAntsNotAtBridge))
  (for _array_element (Variables|Default|GetAnts)
    (Variables|/Game/Blueprints/Core/Swarm/BP_Ant.BP_Ant_C|SetTarget _array_element (Variables|Default|GetBridgeStart))
    (Variables|/Game/Blueprints/Core/Swarm/BP_Ant.BP_Ant_C|SetTargetDistance _array_element 5e+01)
    (Utilities|Array|Add (Variables|Default|GetAntsNotAtBridge) _array_element)))

(fn RemoveBridge
  (params (EndPosition :type Vector))
  (bind _antsnotatbridge (Variables|Default|GetAntsNotAtBridge))
  (if (Variables|Default|GetBridging)
    (Variables|Default|SetBridging false)
    (Variables|Default|SetBridgeEnd EndPosition)
    ;[1 1 1] Set the target of all ants to the target
    (for _array_element (Variables|Default|GetAnts)
      (Variables|/Game/Blueprints/Core/Swarm/BP_Ant.BP_Ant_C|SetTarget _array_element (Variables|Default|GetBridgeEnd)))
    ;[1 1 1] For every ant not at the bridge teleport it to the new target to ensure no ants are left behind
    (bind _arrayelement (Utilities|Array|ReverseforEachLoop _antsnotatbridge)
      (:LoopBody
        (Default|TeleporttoTarget _arrayelement))
      (:Completed
        (Utilities|Array|Clear _antsnotatbridge)))))

(fn UpdateBridge
  (params (End :type Vector) (Start :type Vector))
  (bind _ants (Variables|Default|GetAnts))
  (bind _returnvalue (Utilities|Array|Length _ants))
  (bind _returnvalue_2 (- _returnvalue 1))
  (Variables|Default|SetBridgeEnd End)
  (Variables|Default|SetBridgeStart Start)
  (Utilities|Array|Clear (Variables|Default|GetBridgePositions))
  ;[1 1 1] Calculate the ant positions along the bridge
  (for _index (range 0 _returnvalue_2)
    (Utilities|Array|Add (Variables|Default|GetBridgePositions) (Math|Vector|Lerp(Vector) (Variables|Default|GetBridgeStart) (Variables|Default|GetBridgeEnd) (/ _index _returnvalue_2)))))