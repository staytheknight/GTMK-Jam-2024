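; Tail actor for a swarm, linked to the swarm it spawned from through SwarmSpawnedFrom.
; Shortly after BeginPlay it sets that swarm's HasTail flag.
; While Collapse is true, Tick uses VInterpTo to pull the tail toward the swarm's root location at MovementSpeed.
; Once within MinDistanceToDelete, it clears HasTail and destroys itself.
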(event EventTick
  (params (DeltaSeconds :type Float%20%28single-precision%29))
  (bind _swarmspawnedfrom (Variables|Default|GetSwarmSpawnedFrom))
  (bind _rootcomponent (Variables|/Script/Engine.Actor|GetRootComponent _swarmspawnedfrom))
  (bind _returnvalue (Transformation|GetWorldLocation _rootcomponent))
  (if (Variables|Default|GetCollapse)
    (CallFunction|MovetoTarget _returnvalue DeltaSeconds)
    (if (< (Math|Vector|Distance(Vector) _returnvalue (Transformation|GetWorldLocation (Variables|Default|GetDefaultSceneRoot))) (Variables|Default|GetMinDistanceToDelete))
      (Variables|/Game/Blueprints/Core/Swarm/BP_Swarm.BP_Swarm_C|SetHasTail (Variables|Default|GetSwarmSpawnedFrom) false)
      (Actor|DestroyActor))))

(event EventBeginPlay
  (Utilities|FlowControl|Delay 0.2)
  (Variables|/Game/Blueprints/Core/Swarm/BP_Swarm.BP_Swarm_C|SetHasTail (Variables|Default|GetSwarmSpawnedFrom) true))

(fn ConstructionScript)

(fn MovetoTarget
  (params (Target :type Vector) (DeltaTime :type Float%20%28double-precision%29))
  (bind _defaultsceneroot (Variables|Default|GetDefaultSceneRoot))
  (Transformation|SetWorldLocation _defaultsceneroot (Math|Interpolation|VInterpTo (Transformation|GetWorldLocation _defaultsceneroot) Target DeltaTime (Variables|Default|GetMovementSpeed)) false false))