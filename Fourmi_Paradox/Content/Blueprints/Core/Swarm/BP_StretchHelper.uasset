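; BP_StretchHelper draws a ring of BP_StretchIndicator markers showing the swarm's stretch distance.
; A looping timer spawns 24 markers at Z=0, with radius swarm size times stretch multiplier, when size exceeds one.
; The ring centers on the tail in stretch mode, otherwise on the swarm root if a tail exists.
; An offset looping timer destroys all indicators, so the ring is continually rebuilt by respawning actors.
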(event Custom|Spawn%20Cubes
  (CallFunction|SpawnCubes))

(event Custom|Destroy%20Cubes
  (bind _outactors (Actor|GetAllActorsOfClass "/Game/Blueprints/Core/Swarm/BP_StretchIndicator.BP_StretchIndicator_C"))
  (for _array_element _outactors
    (Utilities|IsValid _array_element
      (:Is%20Valid
        (Actor|DestroyActor _array_element)))))

(event EventBeginPlay
  (Utilities|FlowControl|Sequence
    (:then_0
      (Utilities|FlowControl|Delay 0.2)
      (bind _outactors (Actor|GetAllActorsOfClass "/Game/Blueprints/Core/Player/BP_Pawn.BP_Pawn_C"))
      (Variables|Default|SetBP_Pawn (Utilities|Array|Get(acopy) _outactors)))
    (:then_1
      (Utilities|Time|SetTimerbyEvent (delegate Custom|Spawn%20Cubes) 0.03 true true))
    (:then_2
      (Utilities|Time|SetTimerbyEvent (delegate Custom|Destroy%20Cubes) 0.03 true true 0.03))))

(event EventTick
  (params (DeltaSeconds :type Float%20%28single-precision%29)))

(fn ConstructionScript)

(fn SpawnCubes
  (bind _bp_pawn (Variables|Default|GetBP_Pawn))
  (bind _swarm (Variables|/Game/Blueprints/Core/Player/BP_Pawn.BP_Pawn_C|GetSwarm _bp_pawn))
  (bind _tail (Variables|/Game/Blueprints/Core/Swarm/BP_Swarm.BP_Swarm_C|GetTail _swarm))
  (bind _swarmsize (Variables|/Game/Blueprints/Core/Swarm/BP_Swarm.BP_Swarm_C|GetSwarmSize _swarm))
  (Utilities|IsValid _bp_pawn
    (:Is%20Valid
      (if (> _swarmsize 1)
        (if (Variables|/Game/Blueprints/Core/Swarm/BP_Swarm.BP_Swarm_C|GetStretchMode _swarm)
          (LocalVariables|SetTarget (Variables|/Game/Blueprints/Core/Swarm/BP_Swarm_Tail.BP_Swarm_Tail_C|GetDefaultSceneRoot _tail))
          (else
            (Utilities|IsValid _tail
              (:Is%20Valid
                (LocalVariables|SetTarget (Variables|/Game/Blueprints/Core/Swarm/BP_Swarm.BP_Swarm_C|GetDefaultSceneRoot _swarm))))))
        (for _index (range 0 23)
          (Game|SpawnActorfromClass "/Game/Blueprints/Core/Swarm/BP_StretchIndicator.BP_StretchIndicator_C" (Math|Transform|MakeTransform (Math|Conversions|ToVector(Vector2D) (+ (Class|KismetMathLibrary|GetRotated2D (Math|Vector2D|MakeVector2D (Math|Conversions|ToFloat(Integer) (* _swarmsize (Variables|/Game/Blueprints/Core/Swarm/BP_Swarm.BP_Swarm_C|GetStretchDistanceMultiplier _swarm))) 0.0) (LocalVariables|GetDegreeToRotateBy)) (Math|Vector2D|MakeVector2D (.x (Transformation|GetWorldLocation (LocalVariables|GetTarget))) (.y (Transformation|GetWorldLocation (LocalVariables|GetTarget)))))) (Math|Rotator|MakeRotator 0.0 0.0 (LocalVariables|GetDegreeToRotateBy)) "1.000000,1.000000,1.000000") "AlwaysSpawn" "MultiplyWithRoot" 0 0)
          (if (== (LocalVariables|GetDegreeToRotateBy) 345.0)
            (LocalVariables|SetDegreeToRotateBy 0.0)
            (else
              (LocalVariables|SetDegreeToRotateBy (+ (LocalVariables|GetDegreeIncrease) (LocalVariables|GetDegreeToRotateBy))))))))))