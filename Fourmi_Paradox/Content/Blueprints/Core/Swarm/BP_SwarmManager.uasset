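; Manager actor that keeps a registry of BP_Swarm actors and provides functions to create, split, merge and delete them.
; The construction script gathers existing swarms into SwarmMembers, which creation and deletion then update.
; Splitting moves part of SwarmSize into a new swarm at the same transform, while merging adds sizes and destroys the absorbed swarm.
; Distance queries over the registry return swarms within a radius or the closest other swarm.
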(event EventBeginPlay)

(event Collision|EventActorBeginOverlap
  (params (OtherActor :type Actor%20Object%20Reference)))

(event EventTick
  (params (DeltaSeconds :type Float%20%28single-precision%29)))

(fn ConstructionScript
  (bind _outactors (Actor|GetAllActorsOfClass "/Game/Blueprints/Core/Swarm/BP_Swarm.BP_Swarm_C"))
  (for _array_element _outactors
    (Utilities|Array|Add (Variables|Default|GetSwarmMembers) _array_element)))

(fn CreateSwarm
  (params (SpawnTransform :type Transform) (SwarmSize :type Integer))
  (bind _returnvalue (Game|SpawnActorfromClass "/Game/Blueprints/Core/Swarm/BP_Swarm.BP_Swarm_C" SpawnTransform "Undefined" "MultiplyWithRoot" self SwarmSize 0))
  (Utilities|Array|Add (Variables|Default|GetSwarmMembers) _returnvalue)
  (return _returnvalue))

(fn SplitSwarm
  (params (Swarm :type BP%20Swarm%20Object%20Reference%20%28by%20ref%29) (SplitSwarmSize :type Integer))
  (bind _returnvalue (Transformation|GetActorTransform Swarm))
  (if (> (Variables|/Game/Blueprints/Core/Swarm/BP_Swarm.BP_Swarm_C|GetSwarmSize Swarm) SplitSwarmSize)
    (Variables|/Game/Blueprints/Core/Swarm/BP_Swarm.BP_Swarm_C|SetSwarmSize Swarm (- (Variables|/Game/Blueprints/Core/Swarm/BP_Swarm.BP_Swarm_C|GetSwarmSize Swarm) SplitSwarmSize)) ; Decrease the swarm size of the original swarm
    (bind _swarm (CallFunction|CreateSwarm (Math|Transform|MakeTransform (.location _returnvalue) (.rotation _returnvalue) (.scale _returnvalue)) SplitSwarmSize))
    (return true _swarm)
    (else
      (return false 0))))

(fn MergeSwarms
  (params (Absorber :type BP%20Swarm%20Object%20Reference%20%28by%20ref%29) (Absorbee :type BP%20Swarm%20Object%20Reference%20%28by%20ref%29))
  (Variables|/Game/Blueprints/Core/Swarm/BP_Swarm.BP_Swarm_C|SetSwarmSize Absorber (+ (Variables|/Game/Blueprints/Core/Swarm/BP_Swarm.BP_Swarm_C|GetSwarmSize Absorber) (Variables|/Game/Blueprints/Core/Swarm/BP_Swarm.BP_Swarm_C|GetSwarmSize Absorbee)))
  (CallFunction|DeleteSwarm Absorbee))

(fn DeleteSwarm
  (params (Swarm :type BP%20Swarm%20Object%20Reference%20%28by%20ref%29))
  (if (Utilities|IsValid Swarm)
    (Actor|DestroyActor Swarm)
    (Utilities|Array|RemoveItem (Variables|Default|GetSwarmMembers) Swarm)))

(fn SwarmsinRadius
  (params (Radius :type Float%20%28double-precision%29) (Swarm :type BP%20Swarm%20Object%20Reference))
  (for _array_element (Variables|Default|GetSwarmMembers)
    (if (<= (Transformation|GetDistanceTo _array_element Swarm) Radius)
      (Utilities|Array|Add (LocalVariables|GetInRadius) 0)))
  (return (LocalVariables|GetInRadius)))

(fn GetClosestSwarm
  (params (Swarm :type BP%20Swarm%20Object%20Reference))
  (bind _swarmmembers (Variables|Default|GetSwarmMembers))
  (if (Utilities|Array|IsNotEmpty _swarmmembers)
    (for _array_element _swarmmembers
      ;[1 1 1] make sure the element isn't the same as the passed swarm
      (if (not (== Swarm _array_element))
        (Utilities|IsValid (LocalVariables|GetClosest)
          (:Is%20Valid
            ;[1 1 1] Check if the element is closer to the swarm and if yes update the Closest varaible
            (if (< (Transformation|GetDistanceTo _array_element Swarm) (Transformation|GetDistanceTo (LocalVariables|GetClosest) Swarm))
              (LocalVariables|SetClosest _array_element)))
          (:Is%20Not%20Valid
            (LocalVariables|SetClosest _array_element))))))
  (return (LocalVariables|GetClosest)))