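; Swarm actor that registers with BP_SwarmManager, scaling its physics mesh and merge-detection sphere by swarm size.
; Sphere overlaps track nearby swarms, showing a merge prompt when a controlled one is in range and the pawn's MergeSwarm is this swarm.
; Tick disables gravity in stretch mode, and also physics and collision if uncontrolled.
; It periodically saves the mesh's position to restore it after a fall.
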(event OnComponentEndOverlap(MergeDistanceSphere)
  (params (OverlappedComponent :type Primitive%20Component%20Object%20Reference) (OtherActor :type Actor%20Object%20Reference) (OtherComp :type Primitive%20Component%20Object%20Reference) (OtherBodyIndex :type Integer))
  ;[1 1 1] Adds swarms that are overlapping to an array
  ;;[1 1 1] Ignore self overlaps
  (if (not (== OtherActor self))
    (bind _asbp_swarm (Utilities|Casting|CastToBP_Swarm OtherActor))
    (Utilities|Array|RemoveItem (Variables|Default|GetOverlapList) _asbp_swarm)))

(event OnComponentBeginOverlap(MergeDistanceSphere)
  (params (OverlappedComponent :type Primitive%20Component%20Object%20Reference) (OtherActor :type Actor%20Object%20Reference) (OtherComp :type Primitive%20Component%20Object%20Reference) (OtherBodyIndex :type Integer) (bFromSweep :type Boolean) (SweepResult :type Hit%20Result%20Structure%20%28by%20ref%29))
  ;[1 1 1] Adds swarms that are overlapping to an array
  ;;[1 1 1] Ignore self overlaps
  (if (not (== OtherActor self))
    (bind _asbp_swarm (Utilities|Casting|CastToBP_Swarm OtherActor))
    (Utilities|Array|AddUnique (Variables|Default|GetOverlapList) _asbp_swarm)))

(event EventBeginPlay
  (Utilities|FlowControl|Delay 0.5)
  (bind _outactors (Actor|GetAllActorsOfClass "/Game/Blueprints/Core/Swarm/BP_SwarmManager.BP_SwarmManager_C"))
  (Utilities|Array|Add (Variables|/Game/Blueprints/Core/Swarm/BP_SwarmManager.BP_SwarmManager_C|GetSwarmMembers (Utilities|Array|Get(acopy) _outactors)) self)
  ;[1 1 1] Get BP Pawn to check if self is the merge / closest swarm
  (bind _outactors_2 (Actor|GetAllActorsOfClass "/Game/Blueprints/Core/Player/BP_Pawn.BP_Pawn_C"))
  (Variables|Default|SetBP%20Pawn (Utilities|Array|Get(acopy) _outactors_2)))

(event EventTick
  (params (DeltaSeconds :type Float%20%28single-precision%29))
  (bind _swarmsize (Variables|Default|GetSwarmSize))
  (bind _sm_swarm (Variables|Default|GetSM_Swarm))
  (bind _returnvalue (Class|PrimitiveComponent|IsGravityEnabled _sm_swarm))
  ;[1 1 1] Updates the size of the mesh & overlap element based on swarm size
  (Transformation|SetWorldScale3D (Variables|Default|GetSM_Swarm) (Math|Vector|MakeVector (Math|Conversions|ToFloat(Integer) _swarmsize) (Math|Conversions|ToFloat(Integer) _swarmsize) (Variables|Default|GetDefaultZHeightOfMesh)))
  (Components|Sphere|SetSphereRadius (Variables|Default|GetMerge%20Distance%20Sphere) (* _swarmsize (Variables|Default|GetDefaultSphereRadius)) true)
  (MergePrompt|ToggleMergePrompt)
  (MergePrompt|UpdateMergePromptLocation)
  (CallFunction|ToggleCollisionsOffWhileNotControlled)
  (CallFunction|ResetLocationonFall (Utilities|Time|GetWorldDeltaSeconds))
  ;[1 1 1] Toggles gravity if it's in stretch mode / has a tail
  (if (Variables|Booleans|GetStretchMode)
    (if _returnvalue
      (Physics|SetEnableGravity _sm_swarm false))
    (elif (not _returnvalue)
      (Physics|SetEnableGravity _sm_swarm true))))

(fn ConstructionScript
  (Variables|Default|SetDefaultZHeightOfMesh (.z (Variables|/Script/Engine.SceneComponent|GetRelativeScale3D (Variables|Default|GetSM_Swarm))))
  ;[1 1 1] Saves default sphere radius of dynamic scaling
  (Variables|Default|SetDefaultSphereRadius (Variables|/Script/Engine.SphereComponent|GetSphereRadius (Variables|Default|GetMerge%20Distance%20Sphere self))))

(fn ShowMergePrompt
  (Development|SetHiddeninGame (Variables|Default|GetMergePrompt) false false))

(fn HideMergePrompt
  (Development|SetHiddeninGame (Variables|Default|GetMergePrompt) true false))

(fn ToggleCollisionsOffWhileNotControlled
  (bind _sm_swarm (Variables|Default|GetSM_Swarm))
  (if (and (not (Variables|Booleans|GetControlled)) (Variables|Booleans|GetStretchMode))
    (Physics|SetSimulatePhysics _sm_swarm false)
    (Collision|SetCollisionEnabled _sm_swarm "NoCollision")
    (else
      (Physics|SetSimulatePhysics _sm_swarm true)
      (Collision|SetCollisionEnabled _sm_swarm "QueryAndPhysics")))
  (return))

(fn ResetLocationonFall
  (params (DeltaTime :type Float%20%28double-precision%29))
  (bind _sm_swarm (Variables|Default|GetSM_Swarm))
  (bind _sm_swarm_2 (Variables|Default|GetSM_Swarm))
  (bind _returnvalue (Transformation|GetWorldLocation _sm_swarm))
  (bind (_x _y _z) (Math|Vector|BreakVector _returnvalue))
  (Utilities|FlowControl|Sequence
    (:then_0
      ;[1 1 1] Accumulates seconds passed
      (bind _output_get (Variables|Default|SetAccumulatedSeconds (+ (Variables|Default|GetAccumulatedSeconds) DeltaTime)))
      ;[1 1 1] If greater than x seconds, save world location - and reset accumulator (only records when above a certain y value)
      (if (> _output_get 2.0)
        (if (> _z 1.0)
          (Variables|Default|SetLastLoc (Math|Vector|MakeVector _x _y 4.0))
          (Variables|Default|SetAccumulatedSeconds 0.0))))
    (:then_1
      ;[1 1 1] If the swarm is detected below a certain Y value - reset it to last known location
      (if (< _z -2.5e+02)
        (Transformation|SetWorldLocation _sm_swarm_2 (Variables|Default|GetLastLoc) false true)
        (Physics|SetPhysicsLinearVelocity _sm_swarm_2 "0, 0, 0" false "None")))))

(fn UpdateMergePromptLocation
  (bind _sm_swarm (Variables|Default|GetSM_Swarm))
  (bind _returnvalue (Transformation|GetWorldLocation _sm_swarm))
  (Transformation|SetWorldLocation (Variables|Default|GetMergePrompt) (Math|Vector|MakeVector (.x _returnvalue) (.y _returnvalue) 2e+01) false false))

(fn ToggleMergePrompt
  (Utilities|IsValid (Variables|Default|GetBP%20Pawn)
    (:Is%20Valid
      (Variables|Booleans|SetPlayerInMergeRadius false)
      (for _array_element (Variables|Default|GetOverlapList)
        (if (Variables|BP_Swarm_C|GetControlled _array_element)
          (Variables|Booleans|SetPlayerInMergeRadius true)))
      (if (and (Variables|Booleans|GetPlayerInMergeRadius) (== (Variables|/Game/Blueprints/Core/Player/BP_Pawn.BP_Pawn_C|GetMergeSwarm (Variables|Default|GetBP%20Pawn)) self))
        (MergePrompt|ShowMergePrompt)
        (else
          (MergePrompt|HideMergePrompt))))))