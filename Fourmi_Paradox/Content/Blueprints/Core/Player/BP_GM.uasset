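; Game mode blueprint that bootstraps the swarm game's managers and UI and keeps the on-screen prompts up to date.
; BeginPlay spawns the swarm manager and audio controller, creates the controls and hive widgets, and caches the first hive and pawn found.
; Tick polls pawn swarm count and size to toggle focus, split and stretch instructions, and compares hive food delivered against needed to show the win message.
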(event EventBeginPlay
  (Game|SpawnActorfromClass "/Game/Blueprints/Core/Swarm/BP_SwarmManager.BP_SwarmManager_C" (Math|Transform|MakeTransform "0, 0, 0" "0, 0, 0" "1.000000,1.000000,1.000000") "AlwaysSpawn" "MultiplyWithRoot" 0 0)
  (bind _returnvalue (UserInterface|CreateWidget "/Game/Blueprints/Core/UI/W_GameUI.W_GameUI_C"))
  (Variables|Default|SetControlsUI _returnvalue)
  (UserInterface|Viewport|AddtoViewport _returnvalue 0)
  (bind _returnvalue_2 (UserInterface|CreateWidget "/Game/Blueprints/Core/UI/W_HiveUI.W_HiveUI_C"))
  (Variables|Default|SetW%20Hive%20UI _returnvalue_2)
  (UserInterface|Viewport|AddtoViewport _returnvalue_2 0)
  (bind _outactors (Actor|GetAllActorsOfClass "/Game/Blueprints/Core/Objects/BP_Hive.BP_Hive_C"))
  (Variables|Default|SetBP%20Hive (Utilities|Array|Get(acopy) _outactors))
  (Variables|/Game/Blueprints/Core/UI/W_HiveUI.W_HiveUI_C|SetBP_Hive _returnvalue_2 (Utilities|Array|Get(acopy) _outactors))
  ;[1 1 1] Get Pawn
  (bind _outactors_2 (Actor|GetAllActorsOfClass "/Game/Blueprints/Core/Player/BP_Pawn.BP_Pawn_C"))
  (Variables|Default|SetBP_Pawn (Utilities|Array|Get(acopy) _outactors_2))
  (Game|SpawnActorfromClass "/Game/Audio/BP_AudioController.BP_AudioController_C" (Math|Transform|MakeTransform "0, 0, 0" "0, 0, 0" "1.000000,1.000000,1.000000") "AlwaysSpawn" "MultiplyWithRoot" 0 0))

(event EventTick
  (params (DeltaSeconds :type Float%20%28single-precision%29))
  (CallFunction|UpdateControlsUI)
  (CallFunction|ToggleYouWinMessage))

(fn ConstructionScript)

(fn UpdateControlsUI
  (Utilities|FlowControl|Sequence
    (:then_0
      ;[1 1 1] Toggle Focus Instructions
      (if (> (Utilities|Array|Length (Variables|/Game/Blueprints/Core/Player/BP_Pawn.BP_Pawn_C|GetSwarmList (Variables|Default|GetBP_Pawn))) 1)
        (Variables|/Script/UMG.Widget|SetVisibility (Variables|/Game/Blueprints/Core/UI/W_GameUI.W_GameUI_C|GetVerticalBoxFocus (Variables|Default|GetControlsUI)) "Visible")
        (else
          (Variables|/Script/UMG.Widget|SetVisibility (Variables|/Game/Blueprints/Core/UI/W_GameUI.W_GameUI_C|GetVerticalBoxFocus (Variables|Default|GetControlsUI)) "Collapsed"))))
    (:then_1
      ;[1 1 1] Toggle Split Instructions
      (if (> (Variables|/Game/Blueprints/Core/Swarm/BP_Swarm.BP_Swarm_C|GetSwarmSize (Variables|/Game/Blueprints/Core/Player/BP_Pawn.BP_Pawn_C|GetSwarm (Variables|Default|GetBP_Pawn))) 1)
        (Variables|/Script/UMG.Widget|SetVisibility (Variables|/Game/Blueprints/Core/UI/W_GameUI.W_GameUI_C|GetVerticalBoxSplit (Variables|Default|GetControlsUI)) "Visible")
        (else
          (Variables|/Script/UMG.Widget|SetVisibility (Variables|/Game/Blueprints/Core/UI/W_GameUI.W_GameUI_C|GetVerticalBoxSplit (Variables|Default|GetControlsUI)) "Collapsed"))))
    (:then_2
      ;[1 1 1] Toggle Stretch Instructions
      (if (> (Variables|/Game/Blueprints/Core/Swarm/BP_Swarm.BP_Swarm_C|GetSwarmSize (Variables|/Game/Blueprints/Core/Player/BP_Pawn.BP_Pawn_C|GetSwarm (Variables|Default|GetBP_Pawn))) 1)
        (Variables|/Script/UMG.Widget|SetVisibility (Variables|/Game/Blueprints/Core/UI/W_GameUI.W_GameUI_C|GetVerticalBoxStretch (Variables|Default|GetControlsUI)) "Visible")
        (else
          (Variables|/Script/UMG.Widget|SetVisibility (Variables|/Game/Blueprints/Core/UI/W_GameUI.W_GameUI_C|GetVerticalBoxStretch (Variables|Default|GetControlsUI)) "Collapsed"))))))

(fn ToggleYouWinMessage
  (bind _w_hive_ui (Variables|Default|GetW%20Hive%20UI))
  (bind _bp_hive (Variables|Default|GetBP%20Hive))
  (bind _horizontalboxwinmessage (Variables|/Game/Blueprints/Core/UI/W_HiveUI.W_HiveUI_C|GetHorizontalBoxWinMessage _w_hive_ui))
  (if (< (Variables|/Game/Blueprints/Core/Objects/BP_Hive.BP_Hive_C|GetFoodDelivered _bp_hive) (Variables|/Game/Blueprints/Core/Objects/BP_Hive.BP_Hive_C|GetFoodNeeded _bp_hive))
    (Widget|SetVisibility _horizontalboxwinmessage "Hidden")
    (else
      (Widget|SetVisibility _horizontalboxwinmessage "Visible"))))