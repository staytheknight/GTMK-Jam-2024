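; BP_Pawn is the player pawn that steers one BP_Swarm at a time and carries the camera view above it.
; BeginPlay gathers all swarms, selects the first and centers the pawn on it.
; Axis input sets a force applied each Tick to the swarm's SMSwarm, while the pawn smoothly follows in XY at constant height via VInterpTo.
; F cycles control through the swarms round-robin.
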(event EventBeginPlay
  ;[1 1 1] Sets location of camera on startup (prevents ground clipping)
  (Variables|Movement|SetLocation%20Desired (Transformation|GetActorLocation))
  ;[1 1 1] Grabs the original swarm and sets the camera location to it as well as a reference to the swarm object
  (bind _outactors (Actor|GetAllActorsOfClass "/Game/Blueprints/Core/Swarm/BP_Swarm.BP_Swarm_C"))
  (Variables|Default|SetSwarmList _outactors)
  (bind _output_get (Variables|Default|SetSwarm (Utilities|Array|Get(acopy) _outactors)))
  (Transformation|SetActorLocation (Math|Vector|MakeVector (.x (Transformation|GetActorLocation _output_get)) (.y (Transformation|GetActorLocation _output_get)) (.z (Transformation|GetActorLocation))) false false))

(event EventTick
  (params (DeltaSeconds :type Float%20%28single-precision%29))
  (bind _swarm (Variables|Default|GetSwarm))
  (bind _sm_swarm (Variables|/Game/Blueprints/Core/Swarm/BP_Swarm.BP_Swarm_C|GetSM_Swarm _swarm))
  (bind _returnvalue (Transformation|GetWorldLocation _sm_swarm))
  ;[1 1 1] Updates Location of the swarm it's controlling
  (Physics|AddForce _sm_swarm (Math|Vector|MakeVector (Variables|Movement|GetMove%20Speed%20X) (Variables|Movement|GetMove%20Speed%20Y) 0.0) "None" false)
  ;[1 1 1] Updates position of camera
  (Transformation|SetActorLocation (Math|Interpolation|VInterpTo (Transformation|GetActorLocation) (Math|Vector|MakeVector (.x _returnvalue) (.y _returnvalue) (.z (Transformation|GetActorLocation))) DeltaSeconds (Variables|Movement|GetCameraInterpSpeed)) false false))

(event Input|AxisEvents|InputAxisMoveHorizontally
  (params (AxisValue :type Float%20%28single-precision%29))
  ;[1 1 1] Movement keys
  (Variables|Movement|SetMove%20Speed%20Y (* AxisValue (Variables|Movement|GetMove%20Multiplier))))

(event Input|AxisEvents|InputAxisMoveVertically
  (params (AxisValue :type Float%20%28single-precision%29))
  ;[1 1 1] Movement keys
  (Variables|Movement|SetMove%20Speed%20X (* AxisValue (Variables|Movement|GetMove%20Multiplier))))

(event Input|KeyboardEvents|F
  (params (Key :type Key%20Structure :default "None"))
  (:Pressed
    ;[1 1 1] Switches control between all swarms in round robin fashion - checks if the index is out of bounds and sets it back to 0
    (if (> (+ (Variables|Default|GetSwarmIndex) 1) (- (Utilities|Array|Length (Variables|Default|GetSwarmList)) 1))
      (Variables|Default|SetSwarmIndex 0)
      (else
        (Math|Integer|IncrementInt (Variables|Default|GetSwarmIndex)
          (:%20%20
            _))))
    (Variables|Default|SetSwarm (Utilities|Array|Get(acopy) (Variables|Default|GetSwarmList) (Variables|Default|GetSwarmIndex)))))

(fn ConstructionScript)