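; BP_AudioController is an actor that starts the game's theme music and ambient sound as 2D audio on BeginPlay.
; It stores both spawned audio components, but only the music player's volume is adjusted afterward.
; While MusicPlaying is true, Tick ramps MusicVolume linearly up to full and applies it as the volume multiplier, with no fade-out logic.
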(event EventBeginPlay
  (bind _returnvalue (Audio|SpawnSound2D "/Game/Audio/MS_Theme.MS_Theme" 0.0 1.0 0.0 0 false false))
  (Variables|Default|SetMusicPlayer _returnvalue)
  (bind _returnvalue_2 (Audio|SpawnSound2D "/Game/Audio/MS_Ambiant.MS_Ambiant" 0.4 1.0 0.0 0))
  (Variables|Default|SetAmbiance _returnvalue_2))

(event Collision|EventActorBeginOverlap
  (params (OtherActor :type Actor%20Object%20Reference)))

(event EventTick
  (params (DeltaSeconds :type Float%20%28single-precision%29))
  (if (Variables|Default|GetMusicPlaying)
    (bind _output_get (Variables|Default|SetMusicVolume (Math|Float|Min(Float) (+ (Variables|Default|GetMusicVolume) (* DeltaSeconds 0.2)) 1.0)))
    (Audio|Components|Audio|SetVolumeMultiplier (Variables|Default|GetMusicPlayer) _output_get :!class /Script/Engine.AudioComponent)))

(fn ConstructionScript)